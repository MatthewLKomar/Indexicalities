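; Camera actor that rides a referenced spline actor's path, starting after a short delay and timed by Duration through a timeline.
; Rotation follows the spline until CameraTriggered supplies a look-at point and time, switching to an override rotation while movement continues.
; Two timelines scaled to that time blend the override from the current rotation toward the target, then automatically back to the spline's rotation before releasing it.
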(event `self.ReceiveBeginPlay`
  (bind _splineactor (`self.SplineActor`))
  (`/Engine/EditorBlueprintResources/StandardMacros.IsValid` _splineactor
    (:`Is Valid`
      (set `self.Spline` (`/Game/_Blueprints/BP_Spline.Spline` _splineactor))
      (`self.MoveAlong`))))

(event `MoveAlong`
  (bind _spline (`self.Spline`))
  (bind _returnvalue (`SplineComponent.GetLocationAtDistanceAlongSpline` _spline (`self.Dist`) "World"))
  (`KismetSystemLibrary.Delay` 5.0)
  (`TimelineComponent.SetPlayRate` (`self.Timeline`) (/ 1.0 (`self.Duration`)))
  (bind (_direction _line) (`Timeline|Timeline`)
    (:`Update`
      (set `self.Dist` (`KismetMathLibrary.Lerp` (`self.StartDist`) (`SplineComponent.GetSplineLength` (`self.Spline`)) _line))
      (if (`self.LookGraffiti`)
        (`self.K2_SetActorLocationAndRotation` _returnvalue (`self.RotateVal`))
        (else
          (`self.K2_SetActorLocationAndRotation` _returnvalue (`SplineComponent.GetRotationAtDistanceAlongSpline` _spline (`self.Dist`) "World")))))))

(event `LerpCameraBackToSpline`
  ;[1 1 1] Lerp Camera back to spline
  (bind (_direction _line) (`Timeline|ToSpline` :!via `PlayFromStart`)
    (:`Update`
      (set `self.RotateVal` (`KismetMathLibrary.RLerp` (`self.K2_GetActorRotation`) (`SplineComponent.GetRotationAtDistanceAlongSpline` (`self.Spline`) (`self.Dist`) "World") _line)))
    (:`Finished`
      (set `self.LookGraffiti` false))))

(event `LerpCameraToObject`
  ;[1 1 1] LerpCameraToMesh
  (bind (_direction _line) (`Timeline|ToMesh` :!via `PlayFromStart`)
    (:`Update`
      (set `self.RotateVal` (`KismetMathLibrary.RLerp` (`self.K2_GetActorRotation`) (`KismetMathLibrary.FindLookAtRotation` (`self.K2_GetActorLocation`) (`self.Lookto`)) _line)))
    (:`Finished`
      (`self.CameraUnTrigger`))))

(fn `CameraTriggered`
  (params (Time :type "Float (single-precision)") (Lookto :type "Vector Structure"))
  (set `self.TimeToLook` Time)
  (set `self.Lookto` Lookto)
  (set `self.LookGraffiti` true)
  (`TimelineComponent.SetPlayRate` (`self.Tomesh`) (/ 1.0 (`self.TimeToLook`)))
  (`self.LerpCameraToObject`))

(fn `CameraUnTrigger`
  (set `self.Lookto` (0.0 0.0 0.0))
  (`TimelineComponent.SetPlayRate` (`self.ToSpline`) (/ 1.0 (`self.TimeToLook`)))
  (`self.LerpCameraBackToSpline`))

(fn `UserConstructionScript`)