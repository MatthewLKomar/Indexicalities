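; BP_Graffiti is a placeable graffiti plane that can draw a BP_Camera's attention to itself.
; The construction script sets the plane's scale and material from the Type preset, with Custom using zero scale.
; A looping timer starts on BeginPlay, and CameraTrigger line-traces along the Arrow for a BP_Camera.
; On a hit, it calls CameraTriggered with TimeToLook and its own location, then clears the timer.
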(event `self.ReceiveBeginPlay`
  (bind _returnvalue (`KismetSystemLibrary.K2_SetTimerDelegate` (`|CreateDelegate` :!event `Camera Trigger`) 0.2 true))
  (set `self.Handle` _returnvalue))

(fn `Camera Trigger`
  (bind _arrow (`self.Arrow`))
  (bind _returnvalue (`SceneComponent.K2_GetComponentLocation` _arrow))
  (bind (_outhit _returnvalue_2) (`KismetSystemLibrary.LineTraceSingle` _returnvalue (+ _returnvalue (* (`SceneComponent.GetForwardVector` _arrow) 500.0)) "TraceTypeQuery1"))
  (if _returnvalue_2
    (bind _asbp_camera (cast `/Game/_Blueprints/BP_Camera` (`.HitActor` (`GameplayStatics.BreakHitResult` _outhit))))
    (`/Game/_Blueprints/BP_Camera.CameraTriggered` _asbp_camera (`self.TimeToLook`) (`self.K2_GetActorLocation`))
    (`KismetSystemLibrary.K2_ClearAndInvalidateTimerHandle` (`self.Handle`))))

(fn `UserConstructionScript`
  (switch `/Game/_Blueprints/E_GraffitiType` (`self.Type`)
    (:`NewEnumerator0`
      (`self.SetSizeMaterial` (1.0 1.25 1.0) "/Game/_Assets/Graffiti/MI_AyYo.MI_AyYo"))
    (:`NewEnumerator1`
      (`self.SetSizeMaterial` (1.5 1.0 1.0) "/Game/_Assets/Graffiti/MI_BitchDontKill.MI_BitchDontKill"))
    (:`NewEnumerator2`
      (`self.SetSizeMaterial` (1.5 1.0 1.0) "/Game/_Assets/Graffiti/MI_Campus.MI_Campus"))
    (:`NewEnumerator3`
      (`self.SetSizeMaterial` (1.5 1.0 1.0) "/Game/_Assets/Graffiti/MI_DontLick.MI_DontLick"))
    (:`NewEnumerator4`
      (`self.SetSizeMaterial` (1.5 0.7 1.0) "/Game/_Assets/Graffiti/MI_FF.MI_FF"))
    (:`NewEnumerator5`
      (`self.SetSizeMaterial` (1.0 0.8 1.0) "/Game/_Assets/Graffiti/MI_OrangeThing.MI_OrangeThing"))
    (:`NewEnumerator6`
      (`self.SetSizeMaterial` (1.0 1.5 1.0) "/Game/_Assets/Graffiti/MI_Randomdude.MI_Randomdude"))
    (:`NewEnumerator7`
      (`self.SetSizeMaterial` (1.5 1.5 1.0) "/Game/_Assets/Graffiti/MI_CandyCane.MI_CandyCane"))
    (:`NewEnumerator8`
      (`self.SetSizeMaterial` (0.0 0.0 0.0) "/Game/_Assets/Graffiti/MI_CandyCane.MI_CandyCane"))))